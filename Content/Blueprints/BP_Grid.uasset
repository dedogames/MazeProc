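; BP_Grid is a grid generator that spawns a 2D field of scaled-down actors when play begins.
; BeginPlay moves the Cube to a fixed spot above the world origin, then runs nested loops over H and W.
; Each iteration spawns an actor at its indices multiplied by TileSize, at a constant height, in world space from the origin.
; The spawned class is not specified in the graph, and construction, overlap and tick logic are empty.
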(event `self.ReceiveBeginPlay`
  (`SceneComponent.K2_SetWorldLocation` (`self.Cube`) (0.0 0.0 45.0) false false)
  (for _index (range (+ (`self.H`) 1))
    (set `self.i` _index)
    (for _index_2 (range (+ (`self.W`) 1))
      (set `self.j` _index_2)
      (`|SpawnActorFromClass` "/Game/Blueprints/BP_Mesh.BP_Mesh_C" (`KismetMathLibrary.MakeTransform` (`KismetMathLibrary.MakeVector` (`KismetMathLibrary.Conv_IntToDouble` (* (`self.tileSize`) (`self.i`))) (`KismetMathLibrary.Conv_IntToDouble` (* (`self.tileSize`) (`self.j`))) 15.0) (struct) (0.3 0.3 0.3)) "Undefined" "OverrideRootScale" null null))))

(fn `UserConstructionScript`)